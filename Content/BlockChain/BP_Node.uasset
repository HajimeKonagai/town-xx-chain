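; BP_Node is a blockchain network node actor with its own secp256k1 key pair, transaction pool and chain starting from an origin block.
; Payments become signed transactions broadcast to every BP_Node in its routing table, and balances are summed from the chain.
; Mining runs on Tick with a nonce and reward transaction, though ExecuteMining currently always succeeds.
; Received blocks are appended without validation, stop mining and clear the pool.
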(event `self.ReceiveBeginPlay`
  (`|ExecutionSequence`
    (:`then_0`
      (bind _asbp_player_controller (cast `/Game/CoreClass/BP_PlayerController` (`GameplayStatics.GetPlayerController` 0)))
      (set `self.PlayerControllerRef` _asbp_player_controller)
      (bind _returnvalue (`GameplayStatics.GetActorOfClass` "/Game/CoreClass/TimeManager/BP_TimeManager.BP_TimeManager_C"))
      (set `self.TimeManagerRef` _returnvalue))
    (:`then_1`
      (bind _privatekey (`TSBC_EncryptionFunctionLibrary.Secp256k1_GeneratePrivateKey`))
      (set `self.PrivateKey` _privatekey)
      (bind _publickey (`TSBC_EncryptionFunctionLibrary.Secp256k1_GeneratePublicKey` (`self.PrivateKey`)))
      (set `self.PublicKey` _publickey))
    (:`then_2`
      (`KismetArrayLibrary.Array_Add` (`self.Chain`) (`/Game/BlockChain/BlockChainUtil.OriginBlock` "TheOrigin")))
    (:`then_3`
      (`self.UpdateRouting`))))

(event `self.ReceiveTick`
  (params (DeltaSeconds :type "Float (single-precision)"))
  (bind (_blockwithoutnonce_time _blockwithoutnonce_transactions _blockwithoutnonce_prevhash) (break `/Game/BlockChain/Struct/ST_Block` (`self.MakeBlockForMiningWithoutNonce`)))
  (if (`self.InDuringMining`)
    (bind _issuccess (`self.ExecuteMining`))
    (if _issuccess
      (set `self.InDuringMining` false)
      (bind _returnvalue (`|GenericCreateObject` "/Game/BlockChain/Struct/BlockObject.BlockObject_C" (make `/Game/BlockChain/Struct/ST_Block` (`/Game/CoreClass/TimeManager/BP_TimeManager.GetTime` (`self.TimeManagerRef`)) _blockwithoutnonce_transactions _blockwithoutnonce_prevhash (`self.Nonce`))))
      (`self.Broadcast` true _returnvalue)
      (else
        (set `self.Nonce` (+ (`self.Nonce`) 1))))))

(event `StartMining`
  (if (and (not (`self.InDuringMining`)) (> (`KismetArrayLibrary.Array_Length` (`self.TransactionPool`)) 0))
    (set `self.InDuringMining` true)
    (set `self.Nonce` (`KismetMathLibrary.RandomInteger64` 10000))
    (set `self.ChacheBlockForMiningWithoutNonce` (`/Game/BlockChain/BlockChainUtil.BlockToByteArray` (`self.MakeBlockForMiningWithoutNonce`)))))

(event `Payment`
  (params (Receiver :type "Array of Byte") (Amount :type Integer))
  (bind _signedtransaction (`self.GenerateSignedTransaction` Receiver Amount))
  (bind _returnvalue (`|GenericCreateObject` "/Game/BlockChain/Struct/TransactionObject.TransactionObject_C" _signedtransaction))
  (`self.Broadcast` true _returnvalue))

(event `OnUpdateRoutingTable`
  (bind _outactors (`GameplayStatics.GetAllActorsOfClass` "BP_Node_C"))
  (set `self.RoutingTable` _outactors))

(event `OnBroadCast`
  (params (NewParam :type "Object Object Reference"))
  (`/Game/CoreClass/BP_PlayerController.UpdateUI` (`self.PlayerControllerRef`))
  (`|ExecutionSequence`
    (:`then_0`
      (bind _astransaction_object (cast `/Game/BlockChain/Struct/TransactionObject` NewParam))
      (`KismetArrayLibrary.Array_Add` (`self.TransactionPool`) (`/Game/BlockChain/Struct/TransactionObject.Transaction` _astransaction_object)))
    (:`then_1`
      (bind _asblock_object (cast `/Game/BlockChain/Struct/BlockObject` NewParam))
      (set `self.InDuringMining` false)
      (`KismetArrayLibrary.Array_Add` (`self.Chain`) (`/Game/BlockChain/Struct/BlockObject.Block` _asblock_object))
      (`KismetArrayLibrary.Array_Clear` (`self.TransactionPool`)))))

(fn `Broadcast`
  (params (WithSelf :type Boolean) (ParamObject :type "Object Object Reference"))
  (locals (IsInvalidNode :type Boolean))
  (for _array_element (`self.RoutingTable`)
    (`/Engine/EditorBlueprintResources/StandardMacros.IsValid` _array_element
      (:`Is Valid`
        (if (== self _array_element)
          (if WithSelf
            (`self.OnBroadCast` _array_element ParamObject :!label _label))
          (else
            (goto _label))))
      (:`Is Not Valid`
        (set `local.IsInvalidNode` true))))
  (if (`local.IsInvalidNode`)
    (`self.UpdateRouting`)))

(fn `CalsulateAmoutByPublicKey`
  (params (PublicKey :type "Array of Byte (by ref)"))
  (returns (Amount :type Integer))
  (locals (TotalAmount :type Integer))
  (bind _returnvalue (`TSBC_StringUtilsFunctionLibrary.BytesToString` PublicKey))
  (for _array_element (`self.Chain`)
    (for _array_element_2 (`.Transactions_6_621BFDEE4253D469D645DBBF67F5CF41` (break `/Game/BlockChain/Struct/ST_Block` _array_element))
      (`|ExecutionSequence`
        (:`then_0`
          (if (`KismetStringLibrary.EqualEqual_StrStr` (`TSBC_StringUtilsFunctionLibrary.BytesToString` (`.Sender_12_78488D5A478384341684DAA019571B58` (break `/Game/BlockChain/Struct/ST_Transaction` _array_element_2))) _returnvalue)
            (set `local.TotalAmount` (- (`local.TotalAmount`) (`.Amount_23_AC50759840A5FFD96AF8619FA374EECB` (break `/Game/BlockChain/Struct/ST_Transaction` _array_element_2))))))
        (:`then_1`
          (if (`KismetStringLibrary.EqualEqual_StrStr` (`TSBC_StringUtilsFunctionLibrary.BytesToString` (`.Receiver_14_12F5E524483C89AE808522993144CD96` (break `/Game/BlockChain/Struct/ST_Transaction` _array_element_2))) _returnvalue)
            (set `local.TotalAmount` (+ (`local.TotalAmount`) (`.Amount_23_AC50759840A5FFD96AF8619FA374EECB` (break `/Game/BlockChain/Struct/ST_Transaction` _array_element_2)))))))))
  (return (`local.TotalAmount`)))

(fn `CalsulateMyAmount`
  (returns (Amount :type Integer))
  (bind _amount (`self.CalsulateAmoutByPublicKey` (`self.PublicKey`)))
  (return _amount))

(fn `ExecuteMining`
  (returns (IsSuccess :type Boolean))
  (return true))

(fn `GenerateRewardTransaction`
  (returns (RewardTransactions :type "Array of /Game/BlockChain/Struct/ST_Transaction Structure"))
  (return (`|MakeArray` (make `/Game/BlockChain/Struct/ST_Transaction` (`/Game/CoreClass/TimeManager/BP_TimeManager.GetTime` (`self.TimeManagerRef`)) (`TSBC_StringUtilsFunctionLibrary.StringToBytes` (`self.BlockChainName(RewardSender)`)) (`self.PublicKey`) (`self.REWARD_AMOUNT`)))))

(fn `GenerateSignedTransaction`
  (params (Receiver :type "Array of Byte") (Amount :type Integer))
  (returns (SignedTransaction :type "/Game/BlockChain/Struct/ST_Transaction Structure"))
  (locals (Time :type "/Game/CoreClass/TimeManager/ST_Time Structure"))
  (set `local.Time` (`/Game/CoreClass/TimeManager/BP_TimeManager.GetTime` (`self.TimeManagerRef`)))
  (bind _signature (`TSBC_EncryptionFunctionLibrary.Secp256k1_CreateSignature` (`self.PrivateKey`) (`/Game/BlockChain/BlockChainUtil.HashTransaction` false (make `/Game/BlockChain/Struct/ST_Transaction` (struct) (`self.PublicKey`) Receiver Amount))))
  (return (make `/Game/BlockChain/Struct/ST_Transaction` (`local.Time`) (`self.PublicKey`) Receiver Amount _signature)))

(fn `GetNearestNetworkNode`
  (returns (Node :type "/Game/BlockChain/BP_Node Object Reference"))
  (locals (NodeRef :type "/Game/BlockChain/BP_Node Object Reference") (NearestDistance :type "Float (double-precision)" :default 100000.0))
  (for _array_element (`self.RoutingTable`)
    (`/Engine/EditorBlueprintResources/StandardMacros.IsValid` _array_element
      (:`Is Valid`
        (bind _returnvalue (`self.GetDistanceTo` self _array_element))
        (if (< _returnvalue (`local.NearestDistance`))
          (set `local.NodeRef` _array_element)
          (set `local.NearestDistance` _returnvalue)))))
  (return (`local.NodeRef`)))

(fn `GetNodeName`
  (returns (FamiliarName :type String))
  (bind _nodename (`self.NodeName`))
  (if (`KismetStringLibrary.IsEmpty` _nodename)
    (return (`KismetSystemLibrary.GetDisplayName` self))
    (else
      (return _nodename))))

(fn `MakeBlockForMiningWithoutNonce`
  (returns (BlockWithoutNonce :type "/Game/BlockChain/Struct/ST_Block Structure"))
  (locals (TmpTransactions :type "Array of /Game/BlockChain/Struct/ST_Transaction Structure"))
  (bind _chain (`self.Chain`))
  (bind _output_get (set `local.TmpTransactions` (`self.TransactionPool`)))
  (`KismetArrayLibrary.Array_Append` _output_get (`self.GenerateRewardTransaction`))
  (return (make `/Game/BlockChain/Struct/ST_Block` (struct) (`local.TmpTransactions`) (`/Game/BlockChain/BlockChainUtil.HashBlock` (`|GetArrayItem` _chain (`KismetArrayLibrary.Array_LastIndex` _chain))))))

(fn `ReadChain`)

(fn `ShowBallon`
  (params (Text :type Text))
  (`/Game/ActorComponent/BallonComponent.ShowBallon` (`self.BallonComponent`) Text))

(fn `UpdateRouting`
  (bind _outactors (`GameplayStatics.GetAllActorsOfClass` (`self.NetworkNodeClass`)))
  (for _array_element _outactors
    (bind _asbp_node (cast `/Game/BlockChain/BP_Node` _array_element))
    (`self.OnUpdateRoutingTable` _asbp_node)))

(fn `UserConstructionScript`)