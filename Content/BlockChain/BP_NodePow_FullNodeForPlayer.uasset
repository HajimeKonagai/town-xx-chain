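; Player-specific proof-of-work blockchain full node that adds on-screen feedback to mining and payment actions.
; On BeginPlay it caches the BP_Player pawn controlled by its player controller reference.
; StartMining, Payment and ExecuteMining call their parent implementations, then show a message through that pawn's BallonComponent.
; The success balloon appears only when the parent's ExecuteMining returns true, and that result is passed through.
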(event `self.ReceiveBeginPlay`
  (`parent.ReceiveBeginPlay`)
  (bind _asbp_player (cast `/Game/CoreClass/BP_Player` (`Controller.K2_GetPawn` (`self.PlayerControllerRef`))))
  (set `self.PlayerPawnRef` _asbp_player))

(event `self.StartMining`
  (`parent.StartMining`)
  (`/Game/ActorComponent/BallonComponent.ShowBallon` (`/Game/CoreClass/BP_Player.BallonComponent` (`self.PlayerPawnRef`)) "Mining"))

(event `self.Payment`
  (params (Receiver :type "Array of Byte (by ref)") (Amount :type Integer))
  (`parent.Payment` Receiver Amount)
  (`/Game/ActorComponent/BallonComponent.ShowBallon` (`/Game/CoreClass/BP_Player.BallonComponent` (`self.PlayerPawnRef`)) "PayPay!"))

(fn `ExecuteMining`
  (returns (IsSuccess :type Boolean))
  (bind _issuccess (`parent.ExecuteMining`))
  (if _issuccess
    (`/Game/ActorComponent/BallonComponent.ShowBallon` (`/Game/CoreClass/BP_Player.BallonComponent` (`self.PlayerPawnRef`)) "MiningSuccess!!!!!"))
  (return _issuccess))

(fn `UserConstructionScript`
  (`parent.UserConstructionScript`))