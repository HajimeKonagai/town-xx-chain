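; BP_NodePow_FullNode is a proof-of-work blockchain full node that adds balloon notifications to the mining and payment behavior of its parent class.
; StartMining shows a balloon when mining is not already running and the TransactionPool has entries, then calls the parent.
; Payment calls the parent and shows a balloon, while ExecuteMining announces success only when the parent returns true, passing that result through.
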(event `self.StartMining`
  (if (and (not (`self.InDuringMining`)) (> (`KismetArrayLibrary.Array_Length` (`self.TransactionPool`)) 0))
    (`/Game/ActorComponent/BallonComponent.ShowBallon` (`self.BallonComponent`) "Mining!"))
  (`parent.StartMining`))

(event `self.Payment`
  (params (Receiver :type "Array of Byte (by ref)") (Amount :type Integer))
  (`parent.Payment` Receiver Amount)
  (`/Game/ActorComponent/BallonComponent.ShowBallon` (`self.BallonComponent`) "PayPay!"))

(fn `ExecuteMining`
  (returns (IsSuccess :type Boolean))
  (bind _issuccess (`parent.ExecuteMining`))
  (if _issuccess
    (`/Game/ActorComponent/BallonComponent.ShowBallon` (`self.BallonComponent`) "MiningSuccess!!!!!"))
  (return _issuccess))

(fn `UserConstructionScript`
  (`parent.UserConstructionScript`))