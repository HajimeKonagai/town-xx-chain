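; BP_NodePoW is a blockchain node that performs Proof-of-Work mining, built on a parent node class.
; Its ExecuteMining override calls the parent, hashes the cached block with the current Nonce, and returns whether the hash passes the zero-digit difficulty check.
; Other events only forward to the parent or are disabled, and the "MiningSuccess!!!" balloon message is left unconnected.
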(event `self.ReceiveBeginPlay`
  (`parent.ReceiveBeginPlay`))

(event `self.ReceiveTick`
  (params (DeltaSeconds :type "Float (single-precision)"))
  (`parent.ReceiveTick` DeltaSeconds))

(event `self.OnBroadCast`
  (params (NewParam :type "Object Object Reference"))
  (`parent.OnBroadCast` NewParam))

(fn `ExecuteMining`
  (returns (IsSuccess :type Boolean))
  (`parent.ExecuteMining`)
  (bind _issuccess (`/Game/BlockChain/BlockChainUtil.Is0DigitsInByteArr` (`self.MINING_DIFFICULTY`) (`/Game/BlockChain/BlockChainUtil.HashBlockAddNonce` (`self.ChacheBlockForMiningWithoutNonce`) (`self.Nonce`))))
  (return _issuccess))

(fn `UserConstructionScript`
  (`parent.UserConstructionScript`))