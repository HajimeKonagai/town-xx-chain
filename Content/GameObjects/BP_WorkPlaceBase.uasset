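; Base Blueprint for workplaces that, once placed on a grid cell, process citizens' work every in-game hour via BP_TimeManager.
; Citizens overlapping WorkingBox with the matching action are scored by averaging their four stat ratios against FitParam, with a large negative score beyond Capacity.
; Scores feed CommitWork, then WorkCommited, both empty here.
; BeginPlay also caches the player's BP_NodePoW blockchain node and sums FitParam into a work difficulty.
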(event `self.ReceiveBeginPlay`
  (bind (_fitparam_name _fitparam_power _fitparam_intelligence _fitparam_tech _fitparam_charm) (break `/Game/Character/CitizenParameter` (`self.FitParam`)))
  (`|ExecutionSequence`
    (:`then_0`
      (bind _returnvalue (`GameplayStatics.GetActorOfClass` "/Game/CoreClass/TimeManager/BP_TimeManager.BP_TimeManager_C"))
      (bind _output_get (set `self.TimeManagerRef` _returnvalue))
      (add `/Game/CoreClass/TimeManager/BP_TimeManager.ChangeHour` _output_get (delegate `HourChanged`))
      (bind _asbp_player_controller (cast `/Game/CoreClass/BP_PlayerController` (`GameplayStatics.GetPlayerController` 0)))
      (bind _output_get_2 (set `self.PlayerControllerRef` _asbp_player_controller))
      (bind _asbp_node_po_w (cast `/Game/BlockChain/BP_NodePoW` (`ChildActorComponent.ChildActor` (`/Game/CoreClass/BP_PlayerController.BlockChainNode` _output_get_2))))
      (set `self.NodeRef` _asbp_node_po_w))
    (:`then_1`
      (set `self.WorkDifficality` (+ _fitparam_power _fitparam_intelligence _fitparam_tech _fitparam_charm)))))

(event `HourChanged`
  ; 設置済み
  (`/Engine/EditorBlueprintResources/StandardMacros.IsValid` (`self.GridCell`)
    (:`Is Valid`
      (for _array_element (`self.CitizensByAction` "NewEnumerator2")
        (`self.CommitWork` (`self.CalculateFitting` _array_element) _array_element))
      (`self.WorkCommited`))))

(fn `CalculateFitting`
  (params (Citizen :type "/Game/Character/BP_Citizen Object Reference"))
  (returns (FitRate :type "Float (double-precision)"))
  (bind _workingcitizens (`self.CitizensByAction` "NewEnumerator2"))
  (bind _capacity (`self.Capacity`))
  (bind (_name _power _intelligence _tech _charm) (break `/Game/Character/CitizenParameter` (`self.FitParam`)))
  (bind (_name_2 _power_2 _intelligence_2 _tech_2 _charm_2) (break `/Game/Character/CitizenParameter` (`/Game/Character/BP_Citizen.Param` Citizen)))
  (if (> (`KismetArrayLibrary.Array_Length` _workingcitizens) _capacity)
    (if (and (`KismetArrayLibrary.Array_Contains` _workingcitizens Citizen) (<= (`KismetArrayLibrary.Array_Find` _workingcitizens Citizen) _capacity))
      _
      (else
        (return -10000.0))))
  (return (/ (+ (/ (`KismetMathLibrary.Conv_IntToDouble` _power_2) (`KismetMathLibrary.Conv_IntToDouble` _power)) (/ (`KismetMathLibrary.Conv_IntToDouble` _intelligence_2) (`KismetMathLibrary.Conv_IntToDouble` _intelligence)) (/ (`KismetMathLibrary.Conv_IntToDouble` _tech_2) (`KismetMathLibrary.Conv_IntToDouble` _tech)) (/ (`KismetMathLibrary.Conv_IntToDouble` _charm_2) (`KismetMathLibrary.Conv_IntToDouble` _charm))) 4.0)))

(fn `CitizensByAction`
  (params (Action :type "/Game/Character/CitizenActionType Enum" :default "NewEnumerator2"))
  (returns (WorkingCitizens :type "Array of /Game/Character/BP_Citizen Object Reference"))
  (locals (TmpWorkingCitizens :type "Array of /Game/Character/BP_Citizen Object Reference"))
  (`KismetArrayLibrary.Array_Clear` (`local.TmpWorkingCitizens`))
  (for _array_element (`PrimitiveComponent.GetOverlappingActors` (`self.WorkingBox`) "/Game/Character/BP_Citizen.BP_Citizen_C")
    (bind _asbp_citizen (cast `/Game/Character/BP_Citizen` _array_element :!pure true))
    (if (`|EnumEquality` (`/Game/Character/BP_Citizen.CurrentAction` _asbp_citizen) Action)
      (`KismetArrayLibrary.Array_Add` (`local.TmpWorkingCitizens`) _asbp_citizen)))
  (return (`local.TmpWorkingCitizens`)))

(fn `CommitWork`
  (params (FitValue :type "Float (double-precision)") (Citizen :type "/Game/Character/BP_Citizen Object Reference")))

(fn `UserConstructionScript`)

(fn `WorkCommited`)