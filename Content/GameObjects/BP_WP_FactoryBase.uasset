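; BP_WP_FactoryBase is a factory base Blueprint with a stub for selling stock to citizens.
; Purchase checks that Stock and the buyer's Amount are both above zero, then calls Payment on the citizen's WalletNode with a zero amount.
; The Stock decrement is disconnected, so purchases leave stock unchanged.
; BeginPlay and the construction script only call their parents, while Tick and overlap events are disabled.
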(event `self.ReceiveBeginPlay`
  (`parent.ReceiveBeginPlay`))

(fn `Purchase`
  (params (`Citizen(buyer)` :type "/Game/Character/BP_Citizen Object Reference"))
  (if (and (> (`self.Stock`) 0) (> (`/Game/Character/BP_Citizen.Amount` `Citizen(buyer)`) 0))
    (`/Game/BlockChain/BP_Node.Payment` :`self` (`/Game/Character/BP_Citizen.WalletNode` `Citizen(buyer)`))))

(fn `UserConstructionScript`
  (`parent.UserConstructionScript`))