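; Base workplace Blueprint for a construction site, where citizens contribute work toward a building.
; CommitWork adds each citizen's fit value to the committed workload and pays the hourly wage to their public key through a node reference.
; WorkCommited updates the construction progress widget and, once the workload exceeds the build requirement, occupies the grid cell with the building class.
; Both functions extend parent logic; the event graph holds only disabled stubs.
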(fn `CommitWork`
  (params (FitValue :type "Float (double-precision)") (Citizen :type "/Game/Character/BP_Citizen Object Reference"))
  (`parent.CommitWork` FitValue Citizen)
  (set `self.CommitedWorkload` (+ (`self.CommitedWorkload`) FitValue))
  (`/Game/BlockChain/BP_Node.Payment` (`self.NodeRef`) (`/Game/Character/BP_Citizen.GetPublicKey` Citizen) (`self.HourlyWage`)))

(fn `UserConstructionScript`
  (`parent.UserConstructionScript`))

(fn `WorkCommited`
  (`parent.WorkCommited`)
  (`ProgressBar.SetPercent` (`/Game/GameObjects/Widget/WB_ConstructionProgress.Progress` (cast `/Game/GameObjects/Widget/WB_ConstructionProgress` (`WidgetComponent.GetWidget` (`self.Widget`)) :!pure true)) (/ (`self.CommitedWorkload`) (`self.WorkloadForBuild`)))
  (if (> (`self.CommitedWorkload`) (`self.WorkloadForBuild`))
    (`/Game/CoreClass/Grid/GridCell.Occupy` (`self.GridCell`) (`self.BuildingClass`))))