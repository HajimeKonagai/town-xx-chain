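; BP_TimeManager runs the in-game clock, tracking time of day and a day counter.
; Each Tick advances time by delta seconds times a multiplier from the TimeSpeed setting, so normal speed is one game hour per second.
; The clock wraps at 24 hours to increment the day, and fires a ChangeHour dispatcher whenever the whole hour changes.
; GetTime returns an STTime struct with day, clock fields and an hour-based timestamp.
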(event `self.ReceiveTick`
  (params (DeltaSeconds :type "Float (single-precision)"))
  (`self.UpdateCurrentTimeOfDay` DeltaSeconds))

(fn `GetTime`
  (returns (Time :type "/Game/CoreClass/TimeManager/ST_Time Structure"))
  (bind _currentday (`self.CurrentDay`))
  (bind _currenttimeofday (`self.CurrentTimeOfDay`))
  (bind _returnvalue (* (mod _currenttimeofday 1.0) 60.0))
  (return (make `/Game/CoreClass/TimeManager/ST_Time` _currentday (`KismetMathLibrary.FTrunc` _currenttimeofday) (`KismetMathLibrary.FTrunc` _returnvalue) (`KismetMathLibrary.FTrunc` (* (mod _returnvalue 60.0) 60.0)) (+ (* _currentday 24) (`self.CurrentTimeOfDay`)))))

(fn `UpdateCurrentTimeOfDay`
  (params (DeltaSeconds :type "Float (double-precision)"))
  (locals (StepByTimeSpeed :type "Float (double-precision)") (NextCurrentTimeOfDay :type "Float (double-precision)"))
  (bind _returnvalue (+ (* DeltaSeconds (`local.StepByTimeSpeed`)) (`self.CurrentTimeOfDay`)))
  (`|ExecutionSequence`
    (:`then_0`
      (switch `/Game/CoreClass/TimeManager/TimeSpeed` (`self.TimeSpeed`)
        (:`NewEnumerator0`
          (set `local.StepByTimeSpeed` 1.0))
        (:`NewEnumerator1`
          (set `local.StepByTimeSpeed` 2.0))
        (:`NewEnumerator2`
          (set `local.StepByTimeSpeed` 5.0))))
    (:`then_1`
      (if (>= _returnvalue 24.0)
        (set `local.NextCurrentTimeOfDay` (- _returnvalue 24.0))
        (set `self.CurrentDay` (+ (`self.CurrentDay`) 1))
        (else
          (set `local.NextCurrentTimeOfDay` _returnvalue))))
    (:`then_2`
      ; Dispath Event if hour changed
      (if (!= (`KismetMathLibrary.FFloor` (`self.CurrentTimeOfDay`)) (`KismetMathLibrary.FFloor` (`local.NextCurrentTimeOfDay`)))
        (`self.ChangeHour`)))
    (:`then_3`
      (set `self.CurrentTimeOfDay` (`local.NextCurrentTimeOfDay`)))))

(fn `UserConstructionScript`)