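; Player character Blueprint with a spring-arm camera, handling look, movement and zoom input.
; Look turns controller yaw and sets a clamped spring-arm pitch, while Move follows the control yaw.
; Zoom clamps the arm length, then UpdateMovementSpeed scales the initial walk speed by arm length over ZoomMax, so zooming in slows the player.
; Alternative world-rotation and pitch-dependent zoom nodes are left unconnected.
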(event `self.ReceiveBeginPlay`
  (set `self.InitialMaxWalkSpeed` (`CharacterMovementComponent.MaxWalkSpeed` (`self.CharacterMovement`)))
  (`self.UpdateMovementSpeed`))

(event `Look`
  (params (Value :type "Vector2D Structure"))
  (bind _lookspeed (`self.LookSpeed`))
  (bind (_relativerotation_roll _relativerotation_pitch) (`KismetMathLibrary.BreakRotator` (`SceneComponent.RelativeRotation` (`self.SpringArm`))))
  (`self.AddControllerYawInput` (* Value_X _lookspeed))
  (`SceneComponent.K2_SetRelativeRotation` (`self.SpringArm`) (`KismetMathLibrary.MakeRotator` 0.0 (`KismetMathLibrary.ClampAngle` (+ (* _lookspeed Value_Y) _relativerotation_pitch) (`self.CameraPitchMin`) (`self.CameraPitchMax`))) false false))

(event `Move`
  (params (Value :type "Vector2D Structure"))
  (bind (_returnvalue_roll _returnvalue_pitch _returnvalue_yaw) (`KismetMathLibrary.BreakRotator` (`self.GetControlRotation`)))
  (bind _returnvalue (`KismetMathLibrary.MakeRotator` 0.0 0.0 _returnvalue_yaw))
  (`self.AddMovementInput` (`KismetMathLibrary.GetRightVector` _returnvalue) Value_X)
  (`self.AddMovementInput` (`KismetMathLibrary.GetForwardVector` _returnvalue) Value_Y))

(event `Zoom`
  (params (Value :type "Float (double-precision)"))
  (bind _springarm (`self.SpringArm`))
  (set `SpringArmComponent.TargetArmLength` (`KismetMathLibrary.FClamp` (+ (* Value (`self.ZoomSpeed`)) (`SpringArmComponent.TargetArmLength` _springarm)) (`self.ZoomMin`) (`self.ZoomMax`)) _springarm)
  (`self.UpdateMovementSpeed`))

(fn `UpdateMovementSpeed`
  (set `CharacterMovementComponent.MaxWalkSpeed` (* (`self.InitialMaxWalkSpeed`) (/ (`SpringArmComponent.TargetArmLength` (`self.SpringArm`)) (`self.ZoomMax`))) (`self.CharacterMovement`)))

(fn `UserConstructionScript`)