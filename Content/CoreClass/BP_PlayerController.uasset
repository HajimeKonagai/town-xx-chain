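; Player controller for a grid-building game (Blockchain Kingdom): forwards camera input to BP_Player and handles placeable placement and actor selection.
; Tick traces under the cursor to the nearest GridManager cell, highlights it and snaps the preview placeable there, hiding it far below when occupied.
; Left-click release occupies focused cells with the preview's class; drag multi-cell focus exists, but FocusStarted is never set true.
; UpdateSelectActor toggles ClickableComponents selection and refreshes UI.
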(event `self.ReceiveBeginPlay`
  (`|ExecutionSequence`
    (:`then_0`
      (`EnhancedInputSubsystemInterface.AddMappingContext` (subsystem `EnhancedInputLocalPlayerSubsystem`) "/Game/Input/IMC_BlockchainKingdom.IMC_BlockchainKingdom" 0 (struct)))
    (:`then_1`
      (bind _asbp_player (cast `/Game/CoreClass/BP_Player` (`self.K2_GetPawn`)))
      (set `self.As BP Player` _asbp_player)
      (bind _returnvalue (`GameplayStatics.GetActorOfClass` "/Game/CoreClass/Grid/GridManager.GridManager_C"))
      (set `self.GridManager` _returnvalue))
    (:`then_2`
      (set `self.NodeRef` (cast `/Game/BlockChain/BP_Node` (`ChildActorComponent.ChildActor` (`self.BlockChainNode`)) :!pure true)))))

(event `EnhancedInput|/Game/Input/IA_Look`
  (params (ActionValue :type "Vector2D Structure") (ElapsedSeconds :type "Float (double-precision)") (TriggeredSeconds :type "Float (double-precision)") (InputAction :type "InputAction Object Reference" :default "/Game/Input/IA_Look.IA_Look"))
  ; Movements
  (:`Triggered`
    (if (`self.LookEnabled`)
      (`/Game/CoreClass/BP_Player.Look` (`self.As BP Player`) ActionValue))))

(event `EnhancedInput|/Game/Input/IA_Move`
  (params (ActionValue :type "Vector2D Structure") (ElapsedSeconds :type "Float (double-precision)") (TriggeredSeconds :type "Float (double-precision)") (InputAction :type "InputAction Object Reference" :default "/Game/Input/IA_Move.IA_Move"))
  ; Movements
  (:`Triggered`
    (`/Game/CoreClass/BP_Player.Move` (`self.As BP Player`) ActionValue)))

(event `EnhancedInput|/Game/Input/IA_Zoom`
  (params (ActionValue :type "Float (double-precision)") (ElapsedSeconds :type "Float (double-precision)") (TriggeredSeconds :type "Float (double-precision)") (InputAction :type "InputAction Object Reference" :default "/Game/Input/IA_Zoom.IA_Zoom"))
  ; Movements
  (:`Triggered`
    (`/Game/CoreClass/BP_Player.Zoom` (`self.As BP Player`) ActionValue)))

(event `EnhancedInput|/Game/Input/IA_MouseRight`
  (params (ActionValue :type Boolean) (ElapsedSeconds :type "Float (double-precision)") (TriggeredSeconds :type "Float (double-precision)") (InputAction :type "InputAction Object Reference" :default "/Game/Input/IA_MouseRight.IA_MouseRight"))
  ; Movements
  (:`Started`
    (set `self.LookEnabled` true))
  (:`Completed`
    (set `self.LookEnabled` false)))

(event `EnhancedInput|/Game/Input/IA_MouseLeft`
  (params (ActionValue :type Boolean) (ElapsedSeconds :type "Float (double-precision)") (TriggeredSeconds :type "Float (double-precision)") (InputAction :type "InputAction Object Reference" :default "/Game/Input/IA_MouseLeft.IA_MouseLeft"))
  (bind _placeableactorref (`self.PlaceableActorRef`))
  (bind _gridarray (`/Game/CoreClass/Grid/GridManager.GridArray` (`self.GridManager`)))
  (:`Started`
    ; BK Zoning IA LeftClick
    (set `self.FocusStarted` false))
  (:`Completed`
    (set `self.FocusStarted` false)
    (for _array_element (`self.FocusingGridCellIndexes`)
      (if (`KismetArrayLibrary.Array_IsValidIndex` _gridarray _array_element)
        (`/Engine/EditorBlueprintResources/StandardMacros.IsValid` _placeableactorref
          (:`Is Valid`
            (`/Game/CoreClass/Grid/GridCell.Occupy` (`|GetArrayItem` _gridarray _array_element) (`GameplayStatics.GetObjectClass` _placeableactorref))))))
    (`self.ClearFocusing`)))

(event `self.ReceiveTick`
  (params (DeltaSeconds :type "Float (single-precision)"))
  (bind _placeableactorref (`self.PlaceableActorRef`))
  (`/Engine/EditorBlueprintResources/StandardMacros.IsValid` (`self.GridManager`)
    (:`Is Valid`
      (bind _nearestindex (`self.UpdateFocusingGrid`))
      ; BK Tick Zoning
      (if (`self.FocusStarted`)
        (`KismetArrayLibrary.Array_AddUnique` (`self.FocusingGridCellIndexes`) _nearestindex)
        (else
          (`self.ClearFocusing`)
          (`KismetArrayLibrary.Array_Add` (`self.FocusingGridCellIndexes`) _nearestindex)))
      (for _array_element (`self.FocusingGridCellIndexes`)
        (`/Engine/EditorBlueprintResources/StandardMacros.IsValid` (`self.PlaceableActorRef`)
          (:`Is Valid`
            (bind _output (`|GetArrayItem` (`/Game/CoreClass/Grid/GridManager.GridArray` (`self.GridManager`)) _array_element))
            (`/Engine/EditorBlueprintResources/StandardMacros.IsValid` (`/Game/CoreClass/Grid/GridCell.OccupingActor` _output)
              (:`Is Valid`
                (`self.K2_SetActorLocation` _placeableactorref (0.0 0.0 -100000.0) false false))
              (:`Is Not Valid`
                (`self.K2_SetActorLocation` _placeableactorref (`self.K2_GetActorLocation` _output) false false)
                (`/Game/CoreClass/Grid/GridCell.ChangeFocusingZoneType` _output (`self.ZoneTypeMode`))))))))))

(fn `ClearFocusing`
  (bind _gridarray (`/Game/CoreClass/Grid/GridManager.GridArray` (`self.GridManager`)))
  (for _array_element (`self.FocusingGridCellIndexes`)
    (if (`KismetArrayLibrary.Array_IsValidIndex` _gridarray _array_element)
      (`/Game/CoreClass/Grid/GridCell.ChangeFocusingZoneType` (`|GetArrayItem` _gridarray _array_element) "NewEnumerator0")))
  (`KismetArrayLibrary.Array_Clear` (`self.FocusingGridCellIndexes`)))

(fn `DetectUIState`
  (returns (UIState :type "/Game/UI/UIStateType Enum"))
  (return "NewEnumerator1"))

(fn `UpdateFocusingGrid`
  (returns (NearestIndex :type Integer))
  (bind (_worldlocation _worlddirection) (`self.DeprojectMousePositionToWorld`))
  (bind _gridmanager (`self.GridManager`))
  (bind _outhit (`KismetSystemLibrary.LineTraceSingle` _worldlocation (+ _worldlocation (* _worlddirection 10000.0)) "TraceTypeQuery3"))
  (bind (_bblockinghit _binitialoverlap _time _distance _location _impactpoint) (`GameplayStatics.BreakHitResult` _outhit))
  (if _bblockinghit
    (bind _nearestindex (`/Game/CoreClass/Grid/GridManager.GetNearestGridIndex` _gridmanager _impactpoint))
    (if (`KismetArrayLibrary.Array_IsValidIndex` (`/Game/CoreClass/Grid/GridManager.GridArray` _gridmanager) _nearestindex)
      (return _nearestindex))))

(fn `UpdatePlaceable`
  (params (PlaceableActorClass :type "/Game/GameObjects/BP_PlaceableBase Class Reference"))
  (bind _placeableactorref (`self.PlaceableActorRef`))
  (`/Engine/EditorBlueprintResources/StandardMacros.IsValid` _placeableactorref
    (:`Is Valid`
      (`self.K2_DestroyActor` _placeableactorref))
    (:`Is Not Valid`
      _))
  (bind _returnvalue (`|SpawnActorFromClass` PlaceableActorClass (`KismetMathLibrary.MakeTransform` (0.0 0.0 -100000.0)) "AlwaysSpawn" "MultiplyWithRoot" null null null))
  (set `self.PlaceableActorRef` _returnvalue))

(fn `UpdateSelectActor`
  (params (NewActor :type "Actor Object Reference"))
  (bind _returnvalue (`self.GetComponentByClass` NewActor "/Game/ActorComponent/ClickableComponents.ClickableComponents_C"))
  (bind _selectingactor (`self.SelectingActor`))
  (bind _returnvalue_2 (`self.GetComponentByClass` _selectingactor "/Game/ActorComponent/ClickableComponents.ClickableComponents_C"))
  (`/Engine/EditorBlueprintResources/StandardMacros.IsValid` _selectingactor
    (:`Is Valid`
      (`/Engine/EditorBlueprintResources/StandardMacros.IsValid` _returnvalue_2
        (:`Is Valid`
          (`/Game/ActorComponent/ClickableComponents.UpdateSelected` _returnvalue_2 false))
        (:`Is Not Valid`
          _))
      (if (== _selectingactor NewActor)
        (set `self.UIState` "NewEnumerator2")
        (set `self.SelectingActor` null)
        (`self.UpdateUI`)
        (else
          (set `self.SelectingActor` NewActor :!label _label)
          (`/Engine/EditorBlueprintResources/StandardMacros.IsValid` _returnvalue
            (:`Is Valid`
              (set `self.UIState` "NewEnumerator2")
              (`/Game/ActorComponent/ClickableComponents.UpdateSelected` _returnvalue true)
              (`self.UpdateUI`))))))
    (:`Is Not Valid`
      (goto _label))))

(fn `UserConstructionScript`)