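; BP_WorkManager matches citizens to workplaces through a Hiring event.
; It selection-sorts every BP_WorkPlaceBase by WorkDifficality, inserting each maximum at the front so the easiest comes first.
; For each workplace in that order, GetMostFittedCitizen scans all BP_Citizen actors for the highest CalculateFitting score.
; Hiring does not use the returned citizen, so no assignment happens here.
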(event `Hiring`
  (for _array_element (`self.SortWorkByDifficulity`)
    (`self.GetMostFittedCitizen` _array_element)))

(fn `GetMostFittedCitizen`
  (params (WorkPlace :type "/Game/GameObjects/BP_WorkPlaceBase Object Reference"))
  (returns (MostFitCitizenOrNull :type "/Game/Character/BP_Citizen Object Reference"))
  (locals (MaxFitRate :type "Float (double-precision)") (MostFitCitizen :type "/Game/Character/BP_Citizen Object Reference"))
  (bind _outactors (`GameplayStatics.GetAllActorsOfClass` "/Game/Character/BP_Citizen.BP_Citizen_C"))
  (for _array_element _outactors
    (bind _fitrate (`/Game/GameObjects/BP_WorkPlaceBase.CalculateFitting` WorkPlace _array_element))
    (if (> _fitrate (`local.MaxFitRate`))
      (set `local.MostFitCitizen` _array_element)
      (set `local.MaxFitRate` _fitrate)))
  (return (`local.MostFitCitizen`)))

(fn `SortWorkByDifficulity`
  (returns (WortedWorkPlace :type "Array of /Game/GameObjects/BP_WorkPlaceBase Object Reference"))
  (locals (Copied :type "Array of /Game/GameObjects/BP_WorkPlaceBase Object Reference") (Sorted :type "Array of /Game/GameObjects/BP_WorkPlaceBase Object Reference") (MaxDiff :type Integer) (MaxDiffIndex :type Integer))
  (bind _copied (`local.Copied`))
  (`|ExecutionSequence`
    (:`then_0`
      (bind _outactors (`GameplayStatics.GetAllActorsOfClass` "/Game/GameObjects/BP_WorkPlaceBase.BP_WorkPlaceBase_C"))
      (for _array_element _outactors
        (`KismetArrayLibrary.Array_Add` (`local.Copied`) _array_element)))
    (:`then_1`
      (while (> (`KismetArrayLibrary.Array_Length` _copied) 0)
        (set `local.MaxDiff` 0)
        (set `local.MaxDiffIndex` 0)
        (for (_array_element_2 _array_index) _copied
          (bind _workdifficality (`/Game/GameObjects/BP_WorkPlaceBase.WorkDifficality` _array_element_2))
          (if (> _workdifficality (`local.MaxDiff`))
            (set `local.MaxDiff` _workdifficality)
            (set `local.MaxDiffIndex` _array_index)))
        (`KismetArrayLibrary.Array_Insert` (`local.Sorted`) (`|GetArrayItem` (`local.Copied`) (`local.MaxDiffIndex`)))
        (`KismetArrayLibrary.Array_Remove` (`local.Copied`) (`local.MaxDiffIndex`))))
    (:`then_2`
      (return (`local.Sorted`)))))

(fn `UserConstructionScript`)