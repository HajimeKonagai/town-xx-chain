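; BP_Ballon is an actor that shows a temporary text balloon through a widget component, then destroys itself.
; On BeginPlay it passes its Text to the WB_Ballon widget and plays a timeline whose Size curve drives the widget's render scale.
; The actor is destroyed when the timeline finishes, or immediately if the widget is not a WB_Ballon.
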(event `self.ReceiveBeginPlay`
  (bind _aswb_ballon (cast `/Game/ActorComponent/WB_Ballon` (`WidgetComponent.GetWidget` (`self.Widget`)))
    (:`then`
      (`/Game/ActorComponent/WB_Ballon.SetText` _aswb_ballon (`self.Text`))
      (bind (_direction _size) (`Timeline|Timeline` :!via `PlayFromStart`)
        (:`Update`
          (`Widget.SetRenderScale` (`WidgetComponent.GetWidget` (`self.Widget`)) (`KismetMathLibrary.Conv_DoubleToVector2D` _size)))
        (:`Finished`
          (`self.K2_DestroyActor` :!label _label))))
    (:`CastFailed`
      (goto _label))))

(fn `UserConstructionScript`)