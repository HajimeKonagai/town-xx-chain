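; BP_Citizen is a simulated citizen with health, calories and a proof-of-work wallet balance, shown in a status widget.
; TimeManager hour changes trigger randomly delayed updates that read the balance, burn calories and, at zero calories, drain health until death.
; It then picks work, hunger, sleep or play by priority, announcing switches in balloons.
; Low stats trigger needs, which persist until full, giving hysteresis.
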(event `self.ReceiveBeginPlay`
  (`|ExecutionSequence`
    (:`then_0`
      (bind _returnvalue (`GameplayStatics.GetActorOfClass` "/Game/CoreClass/TimeManager/BP_TimeManager.BP_TimeManager_C"))
      (bind _output_get (set `self.TimeManagerRef` _returnvalue))
      (add `/Game/CoreClass/TimeManager/BP_TimeManager.ChangeHour` _output_get (delegate `ChangeHourHandler`))
      (bind _asbp_node_pow_wallet (cast `/Game/BlockChain/BP_NodePow_Wallet` (`ChildActorComponent.ChildActor` (`self.WalletActor`))))
      (set `self.WalletNode` _asbp_node_pow_wallet)
      (bind _aswb_citizen_status (cast `/Game/Character/Widget/WB_CitizenStatus` (`WidgetComponent.GetWidget` (`self.Widget`))))
      (set `self.WB_SitizenStatusRef` _aswb_citizen_status))
    (:`then_1`
      (`self.UpdateStatusUI`)
      (`self.UpdateActionByStatus`))))

(event `ChangeHourHandler`
  (`KismetSystemLibrary.Delay` (`KismetMathLibrary.RandomFloat`))
  (`self.UpdateStatuses`))

(fn `CheckAmount`
  (returns (Amount :type Integer))
  (bind _amount (`/Game/BlockChain/BP_Node.CalsulateMyAmount` (`self.WalletNode`)))
  (return _amount))

(fn `DetectActionChange`
  (params (CurrentValue :type Integer) (CompareValue :type Integer) (Action :type "/Game/Character/CitizenActionType Enum" :default "NewEnumerator0") (ChatText :type Text))
  (returns (IsReturn :type Boolean))
  (if (< CurrentValue CompareValue)
    (if (not (`|EnumEquality` (`self.CurrentAction`) Action))
      (`/Game/ActorComponent/BallonComponent.ShowBallon` (`self.BallonComponent`) ChatText)
      (set `self.CurrentAction` Action))
    (return true) ; 強制性的に切り替える
    (else
      (return false) ; 必要なし、ほかの action へ
    )))

(fn `GetPublicKey`
  (returns (PublicKey :type "Array of Byte"))
  (return (`/Game/BlockChain/BP_Node.PublicKey` (`self.WalletNode`))))

(fn `UpdateActionByStatus`
  (`|ExecutionSequence`
    (:`then_0`
      (bind _isreturn (`self.DetectActionChange` (`self.Amount`) 5 "NewEnumerator2" "I want to work."))
      (if _isreturn
        (return)
        (else
          (bind _isreturn_2 (`self.DetectActionChange` (`self.Calorie`) 5 "NewEnumerator1" "I'm Hungry"))
          (if _isreturn_2
            (return)
            (else
              (bind _isreturn_3 (`self.DetectActionChange` (`self.Health`) 5 "NewEnumerator0" "I need to sleep...."))
              (if _isreturn_3
                (return)))))))
    (:`then_1`
      (if (`|EnumEquality` (`self.CurrentAction`) "NewEnumerator2")
        (bind _isreturn_4 (`self.DetectActionChange` (`self.Amount`) (`self.MaxParam`) "NewEnumerator2" "I want to work."))
        (if _isreturn_4
          (return)
          (else
            (if (`|EnumEquality` (`self.CurrentAction`) "NewEnumerator1") :!label _label
              (bind _isreturn_5 (`self.DetectActionChange` (`self.Calorie`) (`self.MaxParam`) "NewEnumerator1" "I'm Hungry"))
              (if _isreturn_5
                (return)
                (else
                  (if (`|EnumEquality` (`self.CurrentAction`) "NewEnumerator0") :!label _label_2
                    (bind _isreturn_6 (`self.DetectActionChange` (`self.Health`) (`self.MaxParam`) "NewEnumerator0" "I need to sleep...."))
                    (if _isreturn_6
                      (return)))))
              (else
                (goto _label_2)))))
        (else
          (goto _label))))
    (:`then_2`
      (if (`|EnumInequality` (`self.CurrentAction`) "NewEnumerator3")
        (`/Game/ActorComponent/BallonComponent.ShowBallon` (`self.BallonComponent`) "I'll just keep playing^^")
        (set `self.CurrentAction` "NewEnumerator3")))))

(fn `UpdateStatuses`
  (bind _walletnode (`self.WalletNode`))
  (bind _param_name (break `/Game/Character/CitizenParameter` (`self.Param`)))
  (`|ExecutionSequence`
    (:`then_0`
      (bind _amount (`/Game/BlockChain/BP_Node.CalsulateAmoutByPublicKey` _walletnode (`/Game/BlockChain/BP_Node.PublicKey` _walletnode)))
      (set `self.Amount` _amount)
      (set `self.Calorie` (`KismetMathLibrary.Min` (`KismetMathLibrary.Max` (- (`self.Calorie`) 1)) (`self.MaxParam`)))
      (if (<= (`self.Calorie`) 0)
        (set `self.Health` (- (`self.Health`) 1))
        (if (<= (`self.Health`) 0)
          (`/Game/ActorComponent/BallonComponent.ShowBallon` (`self.BallonComponent`) (`KismetTextLibrary.Conv_StringToText` (`KismetStringLibrary.Concat_StrStr` _param_name " is Dead")))
          (`self.K2_DestroyActor`)
          (return))))
    (:`then_1`
      (`self.UpdateStatusUI`))
    (:`then_2`
      (`self.UpdateActionByStatus`))))

(fn `UpdateStatusUI`
  (bind _param_name (break `/Game/Character/CitizenParameter` (`self.Param`)))
  (`/Game/Character/Widget/WB_CitizenStatus.UpdateStatus` (`self.WB_SitizenStatusRef`) (/ (`KismetMathLibrary.Conv_IntToDouble` (`self.Health`)) (`KismetMathLibrary.Conv_IntToDouble` (`self.MaxParam`))) (/ (`KismetMathLibrary.Conv_IntToDouble` (`self.Calorie`)) (`KismetMathLibrary.Conv_IntToDouble` (`self.MaxParam`))) (`self.Amount`) _param_name))

(fn `UserConstructionScript`)